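; Wheel component for BP_Vehicle that simulates raycast suspension, tire grip, drive and steering.
; On authority only, each tick reads the driver's movement input and yaws steering wheels.
; A downward trace against WorldStatic yields spring compression, with damping and lateral grip derived from the wheel's per-frame movement.
; On a hit, those forces plus forward drive for motor wheels are applied to the vehicle mesh at the wheel's location.
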(event EventBeginPlay
  (bind _asbp_vehicle (Utilities|Casting|CastToBP_Vehicle (Components|GetOwner)))
  (Variables|Default|SetAs%20BP%20Vehicle%201 _asbp_vehicle))

(event EventTick
  (params (DeltaSeconds :type Float%20%28single-precision%29))
  (bind _returnvalue (Transformation|GetWorldLocation))
  (bind _returnvalue_2 (Math|Float|MakeLiteralFloat 2e+01))
  (bind _returnvalue_3 (Math|Vector|GetUpVector))
  (bind _as_bp_vehicle_1 (Variables|Default|GetAs%20BP%20Vehicle%201))
  (bind _restlength (Variables|Default|GetRestLength))
  (bind _offset (Variables|Default|GetOffset))
  (bind _returnvalue_4 (- _restlength _offset))
  (bind _driver (Variables|/Game/Vehicle/BP_Vehicle.BP_Vehicle_C|GetDriver _as_bp_vehicle_1))
  (bind _returnvalue_5 (* _returnvalue_3 _returnvalue_4 -1.0))
  (bind _returnvalue_6 (+ _returnvalue _returnvalue_5 5.0))
  (Networking|SwitchHasAuthority
    (:Authority
      (Utilities|IsValid _driver
        (:Is%20Valid
          (Variables|Default|SetMovementInput (Variables|/Game/ThirdPerson/Blueprints/BP_ThirdPersonCharacter.BP_ThirdPersonCharacter_C|GetMovementInput _driver)))
        (:Is%20Not%20Valid
          (Variables|Default|SetMovementInput "")))
      (CallFunction|Steer)
      (CallFunction|Susp)
      (if (Variables|Default|GetDebug)
        (Rendering|Debug|DrawDebugLine _returnvalue_6 (+ (* (Math|Vector|GetForwardVector) _returnvalue_2) _returnvalue_6) "(R=1.000000,G=0.000000,B=0.000000,A=1.000000)" 0.0 0.0)
        (Rendering|Debug|DrawDebugLine _returnvalue_6 (+ (* (Math|Vector|GetRightVector) _returnvalue_2) _returnvalue_6) "(R=0.000000,G=1.000000,B=0.000000,A=1.000000)" 0.0 0.0)
        (Rendering|Debug|DrawDebugLine _returnvalue_6 (+ (* (Math|Vector|GetUpVector) _returnvalue_2) _returnvalue_6) "(R=0.000000,G=0.000000,B=1.000000,A=1.000000)" 0.0 0.0)))))

(fn Susp
  (bind _returnvalue (Transformation|GetWorldLocation))
  (bind _returnvalue_2 (Math|Vector|GetRightVector))
  (LocalVariables|Setvel (- (Transformation|GetWorldLocation) (Variables|Default|GetLastPos)))
  (Variables|Default|SetLastPos (Transformation|GetWorldLocation))
  (LocalVariables|SetSuspTesholdStartPos _returnvalue)
  (LocalVariables|SetSuspTresholdEndPos (+ _returnvalue (* (Math|Vector|GetUpVector) (Variables|Default|GetRestLength) "-1.000000,-1.000000,-1.000000")))
  (bind (_outhit _returnvalue_3) (Collision|LineTraceForObjects (LocalVariables|GetSuspTesholdStartPos) (LocalVariables|GetSuspTresholdEndPos) (Utilities|Array|MakeArray "ObjectTypeQuery1") false 0 (select (Variables|Default|GetDebug) "ForOneFrame" "None") true "(R=0.931561,G=1.000000,B=0.000000,A=1.000000)" "(R=0.000000,G=0.756992,B=1.000000,A=1.000000)" 0.0))
  (Variables|Default|SetLastOffset (Variables|Default|GetOffset))
  (if _returnvalue_3
    (Variables|Default|SetOffset (- (Variables|Default|GetRestLength) (.Distance (Collision|BreakHitResult _outhit))))
    (LocalVariables|SetSuspSpeed (- (Variables|Default|GetOffset) (Variables|Default|GetLastOffset)))
    (LocalVariables|SetUpForce (* (Math|Vector|GetUpVector) (+ (* (Variables|Default|GetOffset) (Variables|Default|GetStrength)) (* (Math|Vector|DotProduct (Math|Vector|GetUpVector) (LocalVariables|Getvel)) (Variables|Default|GetDamping) -1.0))))
    (LocalVariables|SetRightForce (* (Math|Vector|DotProduct (LocalVariables|Getvel) _returnvalue_2) (Variables|Default|GetGrip) _returnvalue_2 (Variables|Default|GetMass) -1.0 (/ 1.0 (Utilities|Time|GetWorldDeltaSeconds))))
    (if (Variables|Default|GetMotorWheel)
      (LocalVariables|SetForwardForce (* (Math|Vector|GetForwardVector) (Variables|Default|GetSpeed) (.Y (Math|Vector2D|BreakVector2D (Variables|Default|GetMovementInput))))))
    (Class|PrimitiveComponent|AddForceatLocation (Variables|/Script/Engine.StaticMeshActor|GetStaticMeshComponent (Variables|Default|GetAs%20BP%20Vehicle%201)) (+ (LocalVariables|GetUpForce) (LocalVariables|GetRightForce) (LocalVariables|GetForwardForce)) (Transformation|GetWorldLocation) "None")))

(fn Steer
  (if (Variables|Default|GetSteerWheel)
    (LocalVariables|SetSteerAngle (* (.X (Math|Vector2D|BreakVector2D (Variables|Default|GetMovementInput))) (Variables|Default|GetMaxSteer)))
    (Transformation|SetRelativeRotation (Math|Rotator|MakeRotator 0.0 0.0 (LocalVariables|GetSteerAngle)) false false)
    (return)))